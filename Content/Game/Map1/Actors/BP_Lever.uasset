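; BP_Lever is a one-shot interactable lever that counts toward completing the level.
; Interact disables the lever, rotates its mesh and increments Score in GI_Game, sending an interaction message to all BP_Door actors once the validation threshold is reached.
; It then binds a reset event through BP_Gamemode; the lever's reset handler only decrements the score, leaving its rotation and usability unchanged.
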(event `/Game/Game/Common/Interfaces/BPI_Interaction.Interact`
  (if (`self.CanUseLever`)
    (set `self.CanUseLever` false)
    (`SceneComponent.K2_SetRelativeRotation` (`self.SM_Lever`) (struct :`Pitch` -150.0) false false)
    (`|ExecutionSequence`
      (:`then_0`
        (bind _asgi_game (cast `/Game/Game/GI_Game` (`GameplayStatics.GetGameInstance`)))
        (bind _result (`/Engine/EditorBlueprintResources/StandardMacros.IncrementInt` (`/Game/Game/GI_Game.Score` _asgi_game))
          (:`  `
            (bind _output_get (set `/Game/Game/GI_Game.Score` _result _asgi_game))
            (if (>= _output_get (`/Game/Game/GI_Game.ScoreToValidateLevel` _asgi_game))
              (bind _outactors (`GameplayStatics.GetAllActorsOfClass` "/Game/Game/Map1/Actors/BP_Door.BP_Door_C"))
              (for _array_element _outactors
                (if (`KismetSystemLibrary.DoesImplementInterface` _array_element "/Game/Game/Common/Interfaces/BPI_Interaction.BPI_Interaction_C")
                  (message `/Game/Game/Common/Interfaces/BPI_Interaction.Interact` _array_element)))))))
      (:`then_1`
        (bind _asbp_gamemode (cast `/Game/Game/Map1/BP_Gamemode` (`GameplayStatics.GetGameMode`)))
        (add `/Game/Game/Map1/BP_Gamemode.Reset` _asbp_gamemode (delegate `reset`))))))

(event `reset`
  (bind _asgi_game (cast `/Game/Game/GI_Game` (`GameplayStatics.GetGameInstance`)))
  (bind _result (`/Engine/EditorBlueprintResources/StandardMacros.DecrementFloat` (`KismetMathLibrary.Conv_IntToDouble` (`/Game/Game/GI_Game.Score` _asgi_game)))
    (:`  `
      (set `/Game/Game/GI_Game.Score` (`KismetMathLibrary.FTrunc` _result) _asgi_game))))

(fn `UserConstructionScript`)