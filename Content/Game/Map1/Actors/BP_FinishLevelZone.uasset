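; BP_FinishLevelZone is a trigger volume that ends the level when the player enters it.
; On Box overlap by a BP_Player, it adds the player's UIFinishGame widget to the viewport and shows the mouse cursor.
; It then reads minutes and truncated seconds from BP_Gamemode and writes the elapsed time into the widget's Time text.
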(event `self.Box.OnComponentBeginOverlap`
  (params (OverlappedComponent :type "PrimitiveComponent Object Reference") (OtherActor :type "Actor Object Reference") (OtherComp :type "PrimitiveComponent Object Reference") (OtherBodyIndex :type Integer) (bFromSweep :type Boolean) (SweepResult :type "HitResult Structure (by ref)"))
  (bind _asbp_player (cast `/Game/Player/BP_Player` OtherActor))
  (bind _ui_finishgame (`/Game/Player/BP_Player.UI_FinishGame` _asbp_player))
  (`UserWidget.AddToViewport` _ui_finishgame 0)
  (set `PlayerController.bShowMouseCursor` true (`GameplayStatics.GetPlayerController` 0))
  (bind _asbp_gamemode (cast `/Game/Game/Map1/BP_Gamemode` (`GameplayStatics.GetGameMode`)))
  (set `TextBlock.Text` (`KismetTextLibrary.Conv_StringToText` (`KismetStringLibrary.Concat_StrStr` "Time : " (`KismetSystemLibrary.MakeLiteralString` (`KismetStringLibrary.Conv_IntToString` (`/Game/Game/Map1/BP_Gamemode.Minuts` _asbp_gamemode))) " min " (`KismetStringLibrary.Conv_IntToString` (`KismetMathLibrary.FTrunc` (`/Game/Game/Map1/BP_Gamemode.Seconds` _asbp_gamemode))) "sec")) (`/Game/Player/UI/UI_FinishGame.Time` _ui_finishgame)))

(fn `UserConstructionScript`)