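; Game mode for Map1 that runs recurring light toggles, monster spawner triggers and an elapsed-time clock.
; At BeginPlay it messages a random BP_MonsterSpawner through BPI_Interaction and starts a one-second timer counting seconds and minutes.
; A self-rescheduling timer with a randomized delay toggles every BP_Light's lights and emissive material.
; A FlipFlop makes every second toggle message a random spawner again.
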(event `self.ReceiveBeginPlay`
  (`|ExecutionSequence`
    (:`then_0`
      (bind _outactors (`GameplayStatics.GetAllActorsOfClass` "/Game/Game/Map1/Actors/BP_MonsterSpawner.BP_MonsterSpawner_C"))
      (bind _outitem (`KismetArrayLibrary.Array_Random` _outactors))
      (if (`KismetSystemLibrary.DoesImplementInterface` _outitem "/Game/Game/Common/Interfaces/BPI_Interaction.BPI_Interaction_C")
        (message `/Game/Game/Common/Interfaces/BPI_Interaction.Interact` _outitem)))
    (:`then_1`
      (bind _returnvalue (`KismetSystemLibrary.K2_SetTimerDelegate` (delegate `ToggleLights`) (`KismetMathLibrary.RandomFloatInRange` 60.0 80.0) :!label _label))
      (set `self.LightTimer` _returnvalue))
    (:`then_2`
      (`KismetSystemLibrary.K2_SetTimerDelegate` (delegate `CustomEvent`) 1.0 true))))

(event `CustomEvent`
  (bind _result (`/Engine/EditorBlueprintResources/StandardMacros.IncrementFloat` (`self.Seconds`))
    (:`  `
      (bind _output_get (set `self.Seconds` _result))
      (if (>= _output_get 60.0)
        (set `self.Seconds` 0.0)
        (bind _result_2 (`/Engine/EditorBlueprintResources/StandardMacros.IncrementInt` (`self.Minuts`))
          (:`  `
            (set `self.Minuts` _result_2)))))))

(event `ToggleLights`
  (bind _outactors (`GameplayStatics.GetAllActorsOfClass` "/Game/Game/Map1/Actors/BP_Light.BP_Light_C"))
  (for _array_element _outactors
    (`SceneComponent.ToggleVisibility` (`/Game/Game/Map1/Actors/BP_Light.RectLight` _array_element) false)
    (`SceneComponent.ToggleVisibility` (`/Game/Game/Map1/Actors/BP_Light.PointLight` _array_element) false)
    (`/Game/Game/Map1/Actors/BP_Light.ToggleEmissiveMaterial` _array_element))
  (`|ExecutionSequence`
    (:`then_0`
      (`KismetSystemLibrary.K2_ClearAndInvalidateTimerHandle` (`self.LightTimer`))
      (goto _label))
    (:`then_1`
      (`/Engine/EditorBlueprintResources/StandardMacros.FlipFlop`
        (:`B`
          (bind _outactors_2 (`GameplayStatics.GetAllActorsOfClass` "/Game/Game/Map1/Actors/BP_MonsterSpawner.BP_MonsterSpawner_C"))
          (bind _outitem (`KismetArrayLibrary.Array_Random` _outactors_2))
          (if (`KismetSystemLibrary.DoesImplementInterface` _outitem "/Game/Game/Common/Interfaces/BPI_Interaction.BPI_Interaction_C")
            (message `/Game/Game/Common/Interfaces/BPI_Interaction.Interact` _outitem)))))))

(fn `UserConstructionScript`)