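; BP_Monster is a monster that kills and restarts a player who comes within its sphere in clear line of sight.
; BeginPlay stops its audio and starts a looping timer that polls the sphere for overlapping BP_Player actors, in place of Tick or overlap events.
; A Visibility trace from the monster must hit a player before it calls DeadAndRestart and clears the timer.
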(event `self.ReceiveBeginPlay`
  (`AudioComponent.Stop` (`self.Audio`))
  (bind _returnvalue (`KismetSystemLibrary.K2_SetTimerDelegate` (delegate `CheckOverlappedActors`) 0.2 true))
  (set `self.CheckOverlappedActorsTimer` _returnvalue))

(event `CheckOverlappedActors`
  (for _array_element (`PrimitiveComponent.GetOverlappingActors` (`self.Sphere`) "/Game/Player/BP_Player.BP_Player_C")
    (bind _asbp_player (cast `/Game/Player/BP_Player` _array_element))
    (bind _outhit (`KismetSystemLibrary.LineTraceSingle` (`self.K2_GetActorLocation`) (`self.K2_GetActorLocation` _asbp_player) "TraceTypeQuery1"))
    (if (`GameplayStatics.ObjectIsA` (`.HitActor` (`GameplayStatics.BreakHitResult` _outhit)) "/Game/Player/BP_Player.BP_Player_C")
      (`/Game/Player/BP_Player.DeadAndRestart` _asbp_player)
      (`KismetSystemLibrary.K2_ClearAndInvalidateTimerHandle` (`self.CheckOverlappedActorsTimer`)))))

(fn `UserConstructionScript`)