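; AI controller for the monster, apparently a Detour Crowd variant by its name, that runs the BT_Monster behavior tree on BeginPlay.
; AI perception updates for BP_Player write CanSeePlayer and PlayerRef to the blackboard, clearing them when the player is no longer sensed.
; Sensing the player also starts the monster's audio if it is not already playing, and losing them fades it out over a second.
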(event `self.ReceiveBeginPlay`
  (`self.RunBehaviorTree` "/Game/Monster/BehaviorTree/BT_Monster.BT_Monster"))

(event `self.AIPerception.OnTargetPerceptionUpdated`
  (params (Actor :type "Actor Object Reference") (Stimulus :type "AIStimulus Structure"))
  (bind _returnvalue (`self.K2_GetPawn`))
  (bind _returnvalue_2 (`AIBlueprintHelperLibrary.GetBlackboard` _returnvalue))
  (bind _returnvalue_3 (`AIBlueprintHelperLibrary.GetBlackboard` _returnvalue))
  (bind _asbp_player (cast `/Game/Player/BP_Player` Actor))
  (if (`.bSuccessfullySensed` (break `AIStimulus` Stimulus))
    (`BlackboardComponent.SetValueAsBool` _returnvalue_3 "CanSeePlayer" true)
    (`BlackboardComponent.SetValueAsObject` _returnvalue_3 "PlayerRef" _asbp_player)
    (bind _asbp_monster (cast `/Game/Monster/BP_Monster` _returnvalue))
    (bind _audio (`/Game/Monster/BP_Monster.Audio` _asbp_monster))
    (if (not (`AudioComponent.IsPlaying` _audio))
      (`AudioComponent.Play` _audio 0.0))
    (else
      (`BlackboardComponent.SetValueAsBool` _returnvalue_2 "CanSeePlayer" false)
      (`BlackboardComponent.SetValueAsObject` _returnvalue_2 "PlayerRef" null)
      (bind _asbp_monster_2 (cast `/Game/Monster/BP_Monster` _returnvalue))
      (`AudioComponent.FadeOut` (`/Game/Monster/BP_Monster.Audio` _asbp_monster_2) 1.0 0.0 "Linear"))))

(fn `UserConstructionScript`)